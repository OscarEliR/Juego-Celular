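; BP_Piso is a moving floor tile that keeps an endless track going by triggering the creation of new tiles.
; Every tick it shifts its location by the Movimiento vector.
; Overlapping its Box calls CallGenerarTile to generate a tile, then destroys this one after a short delay.
; GetPuntoNuevaTile exposes the Arrow's world transform as the attach point for the next tile.
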(event OnComponentBeginOverlap(Box)
  (params (OverlappedComponent :type Primitive%20Component%20Object%20Reference) (OtherActor :type Actor%20Object%20Reference) (OtherComp :type Primitive%20Component%20Object%20Reference) (OtherBodyIndex :type Integer) (bFromSweep :type Boolean) (SweepResult :type Hit%20Result%20Structure%20%28by%20ref%29))
  (Default|CallGenerarTile)
  (Utilities|FlowControl|Delay 4.0)
  (Actor|DestroyActor))

(event EventBeginPlay)

(event Collision|EventActorBeginOverlap
  (params (OtherActor :type Actor%20Object%20Reference)))

(event EventTick
  (params (DeltaSeconds :type Float%20%28single-precision%29))
  (Transformation|SetActorLocation (- (Transformation|GetActorLocation) (Variables|Default|GetMovimiento)) false false)
  (Utilities|Casting|CastToBP_Instance (Game|GetGameInstance)))

(fn ConstructionScript)

(fn GetPuntoNuevaTile
  (return (Transformation|GetWorldTransform (Variables|Default|GetArrow))))